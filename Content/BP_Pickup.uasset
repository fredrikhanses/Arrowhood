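; Pickup actor that grants an arrow type to the first-person character that overlaps it.
; Once it has finished spawning, the first valid overlap passes its projectile type to the character's TrySetArrowType, guarded by a one-shot flag.
; It then sets a timer by function name on its Spawner to run Spawn Pickup after the respawn time and destroys itself, leaving respawning to the spawner.
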(event `self.ReceiveActorBeginOverlap`
  (params (OtherActor :type "Actor Object Reference"))
  (bind (_asfirst_person_character _bsuccess) (cast `/Game/FirstPersonCPP/Blueprints/FirstPersonCharacter` OtherActor :!pure true))
  (if (`self.FinishedSpawning`)
    (if (and _bsuccess (`self.NotTriggered`))
      (set `self.NotTriggered` false)
      (`/Game/FirstPersonCPP/Blueprints/FirstPersonCharacter.TrySetArrowType` _asfirst_person_character (`self.Projectile Type`))
      (`KismetSystemLibrary.K2_SetTimer` (`self.Spawner`) "Spawn Pickup" (`self.RespawnTime`))
      (`self.K2_DestroyActor`))))

(fn `UserConstructionScript`)