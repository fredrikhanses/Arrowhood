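; BP_CharacterSelection is the actor that sets up local multiplayer character selection and triggers its ready countdown.
; On BeginPlay it creates a widget, then creates a local player per index up to MaxPlayerCount and spawns an actor owned by it at one of four Arrow transforms.
; Tick starts the countdown once when at least two players are ready in the game instance.
; ResetCountdown re-arms that DoOnce gate.
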(event `self.ReceiveBeginPlay`
  ;[1 1 1] Exclude 0 in the index
  (bind _returnvalue (`|CreateWidget` null))
  (`UserWidget.AddToViewport` _returnvalue 0)
  (set `self.CountDown` _ _returnvalue)
  (bind _asbp_gameinstance (cast `` (`GameplayStatics.GetGameInstance`)))
  (set `self.GameInstance` null _asbp_gameinstance)
  (for _index (range (`self.MaxPlayerCount`))
    ;[1 1 1] Spawn player after start point is registered
    (set `self.Index` _index)
    ;[1 1 1] Spawn players/controllers according to Index
    (bind _returnvalue_2 (`GameplayStatics.CreatePlayer` (`self.Index`)))
    (bind _returnvalue_3 (`|SpawnActorFromClass` "" (`SceneComponent.K2_GetComponentToWorld` (select `int` (`self.Index`) :`0` (`self.Arrow`) :`1` (`self.Arrow1`) :`2` (`self.Arrow2`) :`3` (`self.Arrow3`) :!type "SceneComponent Object Reference")) "Undefined" "OverrideRootScale" _returnvalue_2 null)))
  (bind _outactors (`GameplayStatics.GetAllActorsOfClass` null))
  (set `self.bp_characterSelect` _outactors))

(event `self.ReceiveTick`
  (params (DeltaSeconds :type "Float (single-precision)"))
  ;[1 1 1] Reset counter when >1 player is ready
  (if (>= (`/Game/BluePrints/BP_CharacterSelection.HowManyPlayersAreReady` (`.GameInstance` (`self.GameInstance`))) 2)
    (`/Engine/EditorBlueprintResources/StandardMacros.DoOnce` false :!label _label
      (:`Completed`
        (`/Game/BluePrints/UI_Countdown.StartCounter` (`.CountDown` (`self.CountDown`)))))))

(event `ResetCountdown`
  ;[1 1 1] Reset counter when >1 player is ready
  (goto _label :!via `Reset`))

(fn `UserConstructionScript`)