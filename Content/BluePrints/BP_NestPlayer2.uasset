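; BP_NestPlayer2 is a team nest actor for an arrow game, with a trigger, a mesh and a beam.
; After a short delay on BeginPlay, it caches the game mode and its team's two players, then applies blue or yellow materials based on Team2.
; The trigger's overlap event is empty.
; Disconnected logic would bank an overlapping teammate's score into the team total and reset that player's score.
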(event `self.ReceiveBeginPlay`
  (bind _beam (`self.Beam`))
  (bind _team2 (`self.Team2`))
  (`KismetSystemLibrary.Delay` 0.1)
  (bind _asbpgm_gp2_arrow_game_mode (cast `/Game/BluePrints/BPGM_GP2_ArrowGameMode` (`GameplayStatics.GetGameMode`)))
  (bind _output_get (set `self.GameMode` _asbpgm_gp2_arrow_game_mode))
  (set `self.PlayerReferenceP1P2` (`|GetArrayItem` (`/Game/BluePrints/BPGM_GP2_ArrowGameMode.PlayerArray` _output_get) (select `bool` _team2 :`false` (`self.P1`) :`true` (`self.P2`))))
  (set `self.PlayerReferenceP3P4` (`|GetArrayItem` (`/Game/BluePrints/BPGM_GP2_ArrowGameMode.PlayerArray` (`self.GameMode`)) (select `bool` _team2 :`false` (`self.P3`) :`true` (`self.P4`))))
  (if (`self.Team2`)
    (`PrimitiveComponent.SetMaterial` (`self.StaticMesh`) 0 "/Game/StaticMeshes/Blockout/TeamBlue.TeamBlue")
    (`PrimitiveComponent.SetMaterial` _beam 0 "/Game/StaticMeshes/Blockout/TeamBlueEmissive.TeamBlueEmissive")
    (else
      (`PrimitiveComponent.SetMaterial` (`self.StaticMesh`) 0 "/Game/StaticMeshes/Blockout/TeamYellow.TeamYellow")
      (`PrimitiveComponent.SetMaterial` _beam 0 "/Game/StaticMeshes/Blockout/TeamYellowEmissive.TeamYellowEmissive"))))

(event `self.Trigger.OnComponentBeginOverlap`
  (params (OverlappedComponent :type "PrimitiveComponent Object Reference") (OtherActor :type "Actor Object Reference") (OtherComp :type "PrimitiveComponent Object Reference") (OtherBodyIndex :type Integer) (bFromSweep :type Boolean) (SweepResult :type "HitResult Structure (by ref)")))

(fn `UserConstructionScript`)