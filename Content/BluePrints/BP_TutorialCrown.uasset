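; Tutorial crown pickup that appears after enough balloons are shot and ends the tutorial when collected.
; BalloonShot counts hits against WinAmount, then unhides ScorePickup and enables gravity so it drops.
; On overlap by a FirstPersonCharacter, it applies the team outline stencil and vignette, then hides the pickup.
; It then sets TutorialFinished on GI_GameInstance and opens RealMenu after a short delay.
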(event `/Game/BluePrints/BPI_Tutorial.BalloonShot`
  ;[1 1 1] Drop Crown
  (bind _result (`/Engine/EditorBlueprintResources/StandardMacros.IncrementInt` (`self.NumberBalloonsShot`))
    (:`  `
      (if (>= _result (`self.WinAmount`))
        (`SceneComponent.SetHiddenInGame` (`self.ScorePickup`) false false)
        (`PrimitiveComponent.SetEnableGravity` (`self.ScorePickup`) true)))))

(event `self.ScorePickup.OnComponentBeginOverlap`
  (params (OverlappedComponent :type "PrimitiveComponent Object Reference") (OtherActor :type "Actor Object Reference") (OtherComp :type "PrimitiveComponent Object Reference") (OtherBodyIndex :type Integer) (bFromSweep :type Boolean) (SweepResult :type "HitResult Structure (by ref)"))
  ;[1 1 1] Picked up by Player
  (bind _asfirst_person_character (cast `/Game/FirstPersonCPP/Blueprints/FirstPersonCharacter` OtherActor))
  (`PrimitiveComponent.SetCustomDepthStencilValue` (`Character.Mesh` _asfirst_person_character) (`/Game/FirstPersonCPP/Blueprints/FirstPersonCharacter.TeamOutlineStencilValue` _asfirst_person_character))
  (`/Game/FirstPersonCPP/Blueprints/FirstPersonCharacter.SetVignette` _asfirst_person_character true)
  (`SceneComponent.SetHiddenInGame` (`self.ScorePickup`) true false)
  (set `PrimitiveComponent.bGenerateOverlapEvents` false (`self.ScorePickup`))
  (bind _asgi_game_instance (cast `/Game/BluePrints/GI_GameInstance` (`GameplayStatics.GetGameInstance`)))
  (set `/Game/BluePrints/GI_GameInstance.TutorialFinished` true _asgi_game_instance)
  (`KismetSystemLibrary.Delay` 6.0)
  (`GameplayStatics.OpenLevel` "RealMenu"))

(fn `UserConstructionScript`)