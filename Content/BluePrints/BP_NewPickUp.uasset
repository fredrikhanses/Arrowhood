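; BP_NewPickUp is a spinning, respawning arrow pickup that gives the player a normal, ice or bomb arrow type.
; On BeginPlay, Type selects the sphere's material and projectile class, and a timeline increments the sphere's yaw on each update.
; Overlap by FirstPersonCharacter sets its projectile class and special arrow charge, then hides the pickup.
; A hidden flag blocks further pickups until the respawn delay ends.
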(event `self.ReceiveBeginPlay`
  (bind _type (`self.Type`))
  (bind _sphere (`self.Sphere`))
  (`PrimitiveComponent.SetMaterial` (`self.Sphere`) 0 (select `/Game/BluePrints/Enum_ArrowType` _type :`NewEnumerator0` "/Game/StaticMeshes/Placeholder/lambert1.lambert1" :`NewEnumerator1` "/Game/Materials/PlaceholderBlizz.PlaceholderBlizz" :`NewEnumerator2` "/Game/Materials/PlaceholderExplosion.PlaceholderExplosion" :!type "MaterialInterface Object Reference"))
  (bind _output_get (set `self.ProjectileType` (select `/Game/BluePrints/Enum_ArrowType` _type :`NewEnumerator0` "/Game/FirstPersonCPP/Blueprints/BP_ArrowProjectile.BP_ArrowProjectile_C" :`NewEnumerator1` "/Game/FirstPersonCPP/Blueprints/BP_Arrow_Ice.BP_Arrow_Ice_C" :`NewEnumerator2` "/Game/FirstPersonCPP/Blueprints/BP_Arrow_Bomb.BP_Arrow_Bomb_C" :!type "GP2_ArrowProjectile Class Reference")))
  (`Timeline|SpinnyBoy` :`NewTime` 1.0 :!via `PlayFromStart`
    (:`Update`
      (`SceneComponent.K2_SetRelativeRotation` _sphere (`KismetMathLibrary.MakeRotator` (.roll (`SceneComponent.RelativeRotation` _sphere)) (.pitch (`SceneComponent.RelativeRotation` _sphere)) (+ (.yaw (`SceneComponent.RelativeRotation` _sphere)) 1.0)) false false))))

(event `RespawnTimer`
  (`KismetSystemLibrary.Delay` (`self.RespawnTime`))
  (`self.SetActorHiddenInGame` false)
  (set `self.IsHidden` false))

(event `self.Sphere.OnComponentBeginOverlap`
  (params (OverlappedComponent :type "PrimitiveComponent Object Reference") (OtherActor :type "Actor Object Reference") (OtherComp :type "PrimitiveComponent Object Reference") (OtherBodyIndex :type Integer) (bFromSweep :type Boolean) (SweepResult :type "HitResult Structure (by ref)"))
  (if (`self.IsHidden`)
    _
    (elif (== (`GameplayStatics.GetObjectClass` OtherActor) "/Game/FirstPersonCPP/Blueprints/FirstPersonCharacter.FirstPersonCharacter_C")
      (bind _asfirst_person_character (cast `/Game/FirstPersonCPP/Blueprints/FirstPersonCharacter` OtherActor))
      (set `GP2_ArrowCharacter.ProjectileClass` (stale `self.ReceiveBeginPlay` _output_get) _asfirst_person_character)
      (set `/Game/FirstPersonCPP/Blueprints/FirstPersonCharacter.SpecialArrowCharge` (`self.AmmoToGive`) _asfirst_person_character)
      (`self.SetActorHiddenInGame` true)
      (set `self.IsHidden` true)
      (`self.RespawnTimer`)
      (`KismetSystemLibrary.PrintString` "Poop"))))

(fn `UserConstructionScript`)