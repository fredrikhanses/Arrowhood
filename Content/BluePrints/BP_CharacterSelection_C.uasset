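; BP_CharacterSelection_C is a per-player actor that handles readying up on the character selection screen.
; BeginPlay resets the GameInstance ready count and enables selection mode.
; The bottom face button readies players in PlayerIndex order against that count, playing sound, rumble and toggling the player's component visibility by controller ID.
; Outside selection it advances a widget picture; the count increment and timer stop are unconnected.
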(event `whichIndexAmI`
  (params (PlayerIndex :type Integer))
  (set `self.PlayerIndex` PlayerIndex))

(event `self.ReceiveBeginPlay`
  (bind _asbp_gameinstance (cast `` (`GameplayStatics.GetGameInstance`)))
  (set `/Game/BluePrints/BP_CharacterSelection_C.HowManyPlayersAreReady` 0 _asbp_gameinstance)
  (bind _output_get (set `self.GameInstance` _asbp_gameinstance))
  (set `/Game/BluePrints/BP_CharacterSelection_C.CharacterSelection` true _output_get))

(event `Key|Gamepad_FaceButton_Bottom`
  (params (Key :type "Key Structure"))
  ;[1 1 1] Comment
  (:`Pressed`
    (if (`/Game/BluePrints/BP_CharacterSelection_C.CharacterSelection` (`self.GameInstance`))
      (if (== (`self.PlayerIndex`) 0)
        (set `self.IamReady` true :!label _label)
        (`/Engine/EditorBlueprintResources/StandardMacros.DoOnce` false
          (:`Completed`
            (bind _asplayer_controller (cast `PlayerController` (`self.GetController`)))
            (`GameplayStatics.PlaySoundAtLocation` null (0.0 0.0 0.0) (struct) 1.0 1.0 0.0 null null null)
            (`PlayerController.PlayDynamicForceFeedback` (`GameplayStatics.GetPlayerController` 0) 10.0 0.2 true true true true)
            (switch `int` (`GameplayStatics.GetPlayerControllerID` _asplayer_controller)
              (:`Default`
                (`SceneComponent.ToggleVisibility` (`self.Player1`) false :!label _label_2))
              (:`0`
                (goto _label_2))
              (:`1`
                (`SceneComponent.ToggleVisibility` (`self.Player2`) false))
              (:`2`
                (`SceneComponent.ToggleVisibility` (`self.Player3`) false))
              (:`3`
                (`SceneComponent.ToggleVisibility` (`self.Player4`) false)))
            (cast `` (`WidgetComponent.GetUserWidgetObject` (`self.Widget`)))))
        (elif (and (== (`self.PlayerIndex`) 1) (== (`/Game/BluePrints/BP_CharacterSelection_C.HowManyPlayersAreReady` (`self.GameInstance`)) 1))
          (goto _label)
          (elif (and (== (`self.PlayerIndex`) 2) (== (`/Game/BluePrints/BP_CharacterSelection_C.HowManyPlayersAreReady` (`self.GameInstance`)) 2))
            (goto _label)
            (elif (and (== (`self.PlayerIndex`) 3) (== (`/Game/BluePrints/BP_CharacterSelection_C.HowManyPlayersAreReady` (`self.GameInstance`)) 3))
              (goto _label)))))
      (else
        (bind _foundwidgets (`WidgetBlueprintLibrary.GetAllWidgetsOfClass` null))
        (`/Game/BluePrints/UI_Countdown.PictureSwapAddd` _foundwidgets 1)))))

(fn `UserConstructionScript`)