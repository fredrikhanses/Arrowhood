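; Hovering balloon target with a crown that players can lock onto and shoot with arrows.
; A timeline lerps it up and down, swapping endpoints on finish, and it registers with each FirstPersonCharacter's LockTargetComponent.
; The first arrow hit hides the crown and fractures the balloon with radius damage.
; If Activated, it also spawns a score pickup, notifies the GameMode's score widget, stops hovering and unregisters as a target.
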(event `StartTimer`
  ;[1 1 1] HoverTimer
  (bind (_direction _progress) (`Timeline|Timeline_0` :!via `PlayFromStart` :!label _label)
    (:`Update`
      (`self.K2_SetActorLocation` (`KismetMathLibrary.VLerp` (`self.K2_GetActorLocation` self) (`self.TargetLocation`) _progress))
      (if (== (`self.K2_GetActorLocation` self) (`self.TargetLocation`) :`ErrorTolerance` 10.0)
        (`self.Timeline_0__FinishedFunc`)))
    (:`Finished`
      ;[1 1 1] Reverse target location when finished and restart timer
      (set `self.TempLocation` (`self.OriginalLocation`))
      (set `self.OriginalLocation` (`self.TargetLocation`))
      (set `self.TargetLocation` (`self.TempLocation`))
      (`self.StartTimer`))))

(event `StopTimer`
  ;[1 1 1] HoverTimer
  (goto _label :!via `Stop`))

(event `self.ReceiveBeginPlay`
  (bind _returnvalue (`self.K2_GetActorLocation` self))
  ;[1 1 1] Get GameMode and start hover timer
  (bind _asbpgm_gp2_arrow_game_mode (cast `/Game/BluePrints/BPGM_GP2_ArrowGameMode` (`GameplayStatics.GetGameMode`)))
  (set `self.GameMode` _asbpgm_gp2_arrow_game_mode)
  (set `self.OriginalLocation` _returnvalue)
  (set `self.TargetLocation` (+ _returnvalue (`KismetMathLibrary.MakeVector` 0.0 0.0 (`self.HoverHeight`))))
  (`self.StartTimer`)
  (bind _outactors (`GameplayStatics.GetAllActorsOfClass` "/Game/FirstPersonCPP/Blueprints/FirstPersonCharacter.FirstPersonCharacter_C"))
  (for _array_element _outactors
    (`LockTargetComponent2.AddTargetableTarget` (`GP2_ArrowCharacter.LockTargetComponent` _array_element) self)))

(event `self.BalloonTarget_BalloonTarget_DM.OnComponentHit`
  (params (HitComponent :type "PrimitiveComponent Object Reference") (OtherActor :type "Actor Object Reference") (OtherComp :type "PrimitiveComponent Object Reference") (NormalImpulse :type "Vector Structure") (Hit :type "HitResult Structure (by ref)"))
  (bind _balloontarget_balloontarget_dm (`self.BalloonTarget_BalloonTarget_DM`))
  (bind _balloontarget_crown (`self.BalloonTarget_Crown`))
  (bind (_returnvalue_location _returnvalue_rotation) (`KismetMathLibrary.BreakTransform` (`SceneComponent.K2_GetComponentToWorld` (`self.StaticMeshComponent`))))
  ;[1 1 1] Hit by Arrow
  (cast `/Game/FirstPersonCPP/Blueprints/BP_ArrowProjectile` OtherActor)
  (`/Engine/EditorBlueprintResources/StandardMacros.DoOnce` false
    (:`Completed`
      (`SceneComponent.SetVisibility` _balloontarget_crown false false)
      (`PrimitiveComponent.SetCollisionEnabled` _balloontarget_crown "NoCollision")
      (`DestructibleComponent.ApplyRadiusDamage` _balloontarget_balloontarget_dm 2500.0 (`SceneComponent.K2_GetComponentLocation` _balloontarget_balloontarget_dm) 2500.0 2500.0 true)
      (if (`self.bActivated`)
        (`|SpawnActorFromClass` "/Game/BluePrints/BP_ScorePickup.BP_ScorePickup_C" (`KismetMathLibrary.MakeTransform` _returnvalue_location _returnvalue_rotation (3.0 3.0 3.0)) "AlwaysSpawn" "OverrideRootScale" null null)
        (`SceneComponent.SetVisibility` (`self.TargetBeam`) false false)
        (`/Game/BluePrints/UI_Score.CrownWasDropped` (`/Game/BluePrints/BPGM_GP2_ArrowGameMode.Score Widget` (`self.GameMode`)))
        (`self.StopTimer`)
        (bind _outactors (`GameplayStatics.GetAllActorsOfClass` "/Game/FirstPersonCPP/Blueprints/FirstPersonCharacter.FirstPersonCharacter_C"))
        (for _array_element _outactors
          (`LockTargetComponent2.RemoveTargetableTarget` (`GP2_ArrowCharacter.LockTargetComponent` _array_element) self))))))

(fn `UserConstructionScript`)