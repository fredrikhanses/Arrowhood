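; BP_ScorePickup is the crown pickup that awards score and makes the collecting player the carrier.
; After a brief spawn delay, overlap by an unstunned FirstPersonCharacter adds score, enables outline and vignette, calls SetCarrier on the game mode and destroys the pickup.
; A timeout schedules the game mode's SpawnCrown and destroys the pickup, unless any character has touched it, even a stunned one.
; Random launch impulse and SwitchTarget logic are disconnected.
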(event `self.ReceiveBeginPlay`
  ;[1 1 1] Get Game Mode and Launch Crown
  (`self.SetTimer`)
  (bind _asbpgm_gp2_arrow_game_mode (cast `/Game/BluePrints/BPGM_GP2_ArrowGameMode` (`GameplayStatics.GetGameMode`)))
  (set `self.GameMode` _asbpgm_gp2_arrow_game_mode)
  (set `self.CanBePicked` false)
  (`KismetSystemLibrary.Delay` 0.2)
  (set `self.CanBePicked` true))

(event `self.ScorePickup.OnComponentBeginOverlap`
  (params (OverlappedComponent :type "PrimitiveComponent Object Reference") (OtherActor :type "Actor Object Reference") (OtherComp :type "PrimitiveComponent Object Reference") (OtherBodyIndex :type Integer) (bFromSweep :type Boolean) (SweepResult :type "HitResult Structure (by ref)"))
  ;[1 1 1] Picked up by Player
  (if (`self.CanBePicked`)
    (bind _asfirst_person_character (cast `/Game/FirstPersonCPP/Blueprints/FirstPersonCharacter` OtherActor))
    (set `self.PickedUp` true)
    (if (not (`GP2_ArrowCharacter.IsStunned` _asfirst_person_character))
      (`GP2_ArrowCharacter.OnScoreAdded` _asfirst_person_character (`self.Score`))
      (`PrimitiveComponent.SetRenderCustomDepth` (`Character.Mesh` _asfirst_person_character) true)
      (`/Game/FirstPersonCPP/Blueprints/FirstPersonCharacter.SetVignette` _asfirst_person_character true)
      (`/Game/BluePrints/BPGM_GP2_ArrowGameMode.Set Carrier` (`self.GameMode`) _asfirst_person_character true false)
      (`self.K2_DestroyActor`))))

(event `SetTimer`
  (`KismetSystemLibrary.Delay` (`self.TimeUntilRespawn`))
  (if (not (`self.PickedUp`))
    (bind _asbpgm_gp2_arrow_game_mode (cast `/Game/BluePrints/BPGM_GP2_ArrowGameMode` (`GameplayStatics.GetGameMode`)))
    (`|ExecutionSequence`
      (:`then_0`
        (`KismetSystemLibrary.K2_SetTimer` _asbpgm_gp2_arrow_game_mode "SpawnCrown" 1.0))
      (:`then_1`
        (`self.K2_DestroyActor`)))))

(fn `UserConstructionScript`)