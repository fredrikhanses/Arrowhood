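; BP_Blizzard is a short-lived area effect that slows player characters caught in it, excluding the one stored in its Player variable.
; Trigger overlaps pass through an exact-class FirstPersonCharacter check, then call Slow on the character for SlowDuration.
; On BeginPlay it plays an attenuated placeholder snow sound and destroys itself after a brief delay, or sooner if it overlaps a BP_Explosion.
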(event `self.Trigger.OnComponentBeginOverlap`
  (params (OverlappedComponent :type "PrimitiveComponent Object Reference") (OtherActor :type "Actor Object Reference") (OtherComp :type "PrimitiveComponent Object Reference") (OtherBodyIndex :type Integer) (bFromSweep :type Boolean) (SweepResult :type "HitResult Structure (by ref)"))
  ;[1 1 1] Main Thing
  (if (!= OtherActor (`self.Player`))
    (bind _outputpin (`self.IsThisAPlayer` OtherActor)
      (:`true`
        (bind _asfirst_person_character (cast `/Game/FirstPersonCPP/Blueprints/FirstPersonCharacter` _outputpin))
        (`GP2_ArrowCharacter.Slow` _asfirst_person_character (`self.SlowDuration`) 3.0)))))

(event `self.ReceiveActorBeginOverlap`
  (params (OtherActor :type "Actor Object Reference"))
  ;[1 0.7929 0] Game ends itself if Explosion actor touches it
  (if (== (`GameplayStatics.GetObjectClass` OtherActor) "/Game/BluePrints/BP_Explosion.BP_Explosion_C")
    (`self.K2_DestroyActor`)))

(event `self.ReceiveBeginPlay`
  (`GameplayStatics.PlaySoundAtLocation` "/Game/Sound/Placeholdersnowthing.Placeholdersnowthing" (`SceneComponent.K2_GetComponentLocation` (`self.DefaultSceneRoot`)) (struct) 1.0 1.0 0.0 "/Game/Sound/SpecialArrowAttenuationThing.SpecialArrowAttenuationThing" null null)
  (`KismetSystemLibrary.Delay` 0.2)
  (`self.K2_DestroyActor`))

(fn `UserConstructionScript`)