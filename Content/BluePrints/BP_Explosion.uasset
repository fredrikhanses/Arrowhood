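; BP_Explosion is a short-lived explosion actor that plays a sound on spawn, then destroys itself after a brief delay.
; Its Sphere overlap launches any FirstPersonCharacter strongly upward, with a small horizontal push along the sweep's impact normal.
; A separate KillTrigger overlap kills characters other than the stored Player, crediting Player as killer and passing a normalized force vector pointing toward the explosion.
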(event `self.Sphere.OnComponentBeginOverlap`
  (params (OverlappedComponent :type "PrimitiveComponent Object Reference") (OtherActor :type "Actor Object Reference") (OtherComp :type "PrimitiveComponent Object Reference") (OtherBodyIndex :type Integer) (bFromSweep :type Boolean) (SweepResult :type "HitResult Structure (by ref)"))
  ;[1 0.6714 0.02372] KnockBack Stuff
  (if (== (`GameplayStatics.GetObjectClass` OtherActor) "/Game/FirstPersonCPP/Blueprints/FirstPersonCharacter.FirstPersonCharacter_C")
    (bind _asfirst_person_character (cast `/Game/FirstPersonCPP/Blueprints/FirstPersonCharacter` OtherActor)
      (:`then`
        (`Character.LaunchCharacter` _asfirst_person_character (`KismetMathLibrary.MakeVector` (* (.x (`.ImpactNormal` (`GameplayStatics.BreakHitResult` SweepResult))) 100.0) (* (.y (`.ImpactNormal` (`GameplayStatics.BreakHitResult` SweepResult))) 100.0) (* (.z (`self.GetActorUpVector` _asfirst_person_character)) 1500.0)) false false))
      (:`CastFailed`
        (`KismetSystemLibrary.PrintString` "Cast failed")))))

(event `self.ReceiveBeginPlay`
  ;[1 1 1] Lifetime
  (`GameplayStatics.PlaySoundAtLocation` "/Game/Sound/Explosion01.Explosion01" (0.0 0.0 0.0) (struct) 0.3 1.0 0.0 null null null)
  (`KismetSystemLibrary.Delay` 1.0)
  (`self.K2_DestroyActor`))

(event `self.KillTrigger.OnComponentBeginOverlap`
  (params (OverlappedComponent :type "PrimitiveComponent Object Reference") (OtherActor :type "Actor Object Reference") (OtherComp :type "PrimitiveComponent Object Reference") (OtherBodyIndex :type Integer) (bFromSweep :type Boolean) (SweepResult :type "HitResult Structure (by ref)"))
  (bind _player (`self.Player`))
  ;[1 0 0] Kills Player
  (if (== (`GameplayStatics.GetObjectClass` OtherActor) "/Game/FirstPersonCPP/Blueprints/FirstPersonCharacter.FirstPersonCharacter_C")
    (bind _asfirst_person_character (cast `/Game/FirstPersonCPP/Blueprints/FirstPersonCharacter` OtherActor))
    (if (!= _player _asfirst_person_character)
      (bind _asfirst_person_character_2 (cast `/Game/FirstPersonCPP/Blueprints/FirstPersonCharacter` _player))
      (`/Game/FirstPersonCPP/Blueprints/FirstPersonCharacter.Kill` _asfirst_person_character _asfirst_person_character_2 (`KismetMathLibrary.Normal` (- (`self.K2_GetActorLocation`) (`self.K2_GetActorLocation` _asfirst_person_character)))))))

(fn `UserConstructionScript`)