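; Tutorial balloon target that hovers vertically until an arrow projectile shatters it.
; A looping timeline lerps it between its start and HoverHeight offset, swapping endpoints on each finish.
; The first arrow hit after FinishedSpawning notifies the TutorialCrown found via BPI_Tutorial and schedules SpawnBalloon on the spawner.
; It also spawns a respawn countdown actor, applies radius damage to its destructible mesh and stops hovering.
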(event `StartTimer`
  ;[1 1 1] HoverTimer
  (bind (_direction _progress) (`Timeline|Timeline_0` :!via `PlayFromStart` :!label _label)
    (:`Update`
      (`self.K2_SetActorLocation` (`KismetMathLibrary.VLerp` (`self.K2_GetActorLocation` self) (`self.TargetLocation`) _progress))
      (if (== (`self.K2_GetActorLocation` self) (`self.TargetLocation`) :`ErrorTolerance` 10.0)
        (`self.Timeline_0__FinishedFunc`)))
    (:`Finished`
      ;[1 1 1] Reverse target when finished and restart timer
      (set `self.TempLocation` (`self.OriginalLocation`))
      (set `self.OriginalLocation` (`self.TargetLocation`))
      (set `self.TargetLocation` (`self.TempLocation`))
      (`self.StartTimer`))))

(event `StopTimer`
  ;[1 1 1] HoverTimer
  (goto _label :!via `Stop`))

(event `self.ReceiveBeginPlay`
  (bind _returnvalue (`self.K2_GetActorLocation` self))
  ;[1 1 1] Get Crown reference and start hover timer
  (bind _outactors (`GameplayStatics.GetAllActorsWithInterface` "/Game/BluePrints/BPI_Tutorial.BPI_Tutorial_C"))
  (bind _asbp_tutorial_crown (cast `/Game/BluePrints/BP_TutorialCrown` (`|GetArrayItem` _outactors)))
  (set `self.TutorialCrown` _asbp_tutorial_crown)
  (set `self.OriginalLocation` _returnvalue)
  (set `self.TargetLocation` (+ _returnvalue (`KismetMathLibrary.MakeVector` 0.0 0.0 (`self.HoverHeight`))))
  (`self.StartTimer`))

(event `self.BalloonTarget_BalloonTarget_DM.OnComponentHit`
  (params (HitComponent :type "PrimitiveComponent Object Reference") (OtherActor :type "Actor Object Reference") (OtherComp :type "PrimitiveComponent Object Reference") (NormalImpulse :type "Vector Structure") (Hit :type "HitResult Structure (by ref)"))
  (bind _balloontarget_balloontarget_dm (`self.BalloonTarget_BalloonTarget_DM`))
  ;[1 1 1] Hit by Arrow
  (cast `GP2_ArrowProjectile` OtherActor)
  (if (`self.FinishedSpawning`)
    (`/Engine/EditorBlueprintResources/StandardMacros.DoOnce` false
      (:`Completed`
        (message `/Game/BluePrints/BPI_Tutorial.BalloonShot` (`self.TutorialCrown`))
        (`KismetSystemLibrary.K2_SetTimer` (`self.TutorialBalloonSpawner`) "SpawnBalloon" (`self.RespawnTime`))
        (bind _returnvalue (`|SpawnActorFromClass` "/Game/BP_RespawnCounter.BP_RespawnCounter_C" (`self.GetTransform`) "Undefined" "OverrideRootScale" null null))
        (set `/Game/BP_RespawnCounter.TimeUntilRespawn` (`self.RespawnTime`) _returnvalue)
        (`DestructibleComponent.ApplyRadiusDamage` _balloontarget_balloontarget_dm 2500.0 (`SceneComponent.K2_GetComponentLocation` _balloontarget_balloontarget_dm) 2500.0 2500.0 true)
        (`self.StopTimer`)))))

(fn `UserConstructionScript`)