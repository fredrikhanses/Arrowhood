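; BP_Spawner is a placeable spawner for arrow pickups, set by pickup type to normal, ice or bomb arrows.
; Its construction script previews the chosen mesh and material on an Arrow component, which is destroyed on BeginPlay.
; BeginPlay resolves the projectile class and calls SpawnPickup, which spawns a BP_Pickup at the root transform.
; The pickup receives amount, projectile, visuals, pawn overlap response and a reference back to the spawner.
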(event `self.ReceiveBeginPlay`
  (`ActorComponent.K2_DestroyComponent` (`self.Arrow`))
  (set `self.ProjectileType` (select `/Game/BluePrints/Enum_ArrowType` (`self.PickupType`) :`NewEnumerator0` "/Game/FirstPersonCPP/Blueprints/BP_ArrowProjectile.BP_ArrowProjectile_C" :`NewEnumerator1` "/Game/FirstPersonCPP/Blueprints/BP_Arrow_Ice.BP_Arrow_Ice_C" :`NewEnumerator2` "/Game/FirstPersonCPP/Blueprints/BP_Arrow_Bomb.BP_Arrow_Bomb_C" :!type "/Game/FirstPersonCPP/Blueprints/BP_ArrowProjectile Class Reference"))
  (`self.Spawn Pickup`))

(fn `Spawn Pickup`
  (bind _returnvalue (`|SpawnActorFromClass` "/Game/BP_Pickup.BP_Pickup_C" (`SceneComponent.K2_GetComponentToWorld` (`self.DefaultSceneRoot`)) "AlwaysSpawn" "OverrideRootScale" null null))
  (set `/Game/BP_Pickup.PickupAmount` (`self.PickupAmount`) _returnvalue)
  (set `/Game/BP_Pickup.Spawner` self _returnvalue)
  (set `/Game/BP_Pickup.Projectile Type` (`self.ProjectileType`) _returnvalue)
  (bind _cube (`/Game/BP_Pickup.Cube` _returnvalue))
  (`PrimitiveComponent.SetCollisionResponseToChannel` _cube "ECC_Pawn" "ECR_Overlap")
  (`PrimitiveComponent.SetMaterial` _cube 0 (select `/Game/BluePrints/Enum_ArrowType` (`self.PickupType`) :`NewEnumerator0` "/Engine/EngineDebugMaterials/VertexColorViewMode_ColorOnly.VertexColorViewMode_ColorOnly" :`NewEnumerator1` "/Game/StaticMeshes/Blockout/TeamBlueEmissive.TeamBlueEmissive" :`NewEnumerator2` "/Engine/TemplateResources/MI_Template_BaseOrange.MI_Template_BaseOrange" :!type "MaterialInterface Object Reference"))
  (set `/Game/BP_Pickup.FinishedSpawning` true _returnvalue)
  (`StaticMeshComponent.SetStaticMesh` (`/Game/BP_Pickup.Cube` _returnvalue) (select `/Game/BluePrints/Enum_ArrowType` (`self.PickupType`) :`NewEnumerator0` "/Game/FirstPersonCPP/Anims/SM_Arrow_01.SM_Arrow_01" :`NewEnumerator1` "/Game/StaticMeshes/Arrows/ArrowBundle_Ice.ArrowBundle_Ice" :`NewEnumerator2` "/Game/StaticMeshes/Arrows/ArrowBundle_Bomb.ArrowBundle_Bomb" :!type "StaticMesh Object Reference")))

(fn `UserConstructionScript`
  (bind _pickuptype (`self.PickupType`))
  (`StaticMeshComponent.SetStaticMesh` (`self.Arrow`) (select `/Game/BluePrints/Enum_ArrowType` _pickuptype :`NewEnumerator0` "/Game/FirstPersonCPP/Anims/SM_Arrow_01.SM_Arrow_01" :`NewEnumerator1` "/Game/StaticMeshes/Arrows/ArrowBundle_Ice.ArrowBundle_Ice" :`NewEnumerator2` "/Game/StaticMeshes/Arrows/ArrowBundle_Bomb.ArrowBundle_Bomb" :!type "StaticMesh Object Reference"))
  (`PrimitiveComponent.SetMaterial` (`self.Arrow`) 0 (select `/Game/BluePrints/Enum_ArrowType` _pickuptype :`NewEnumerator0` "/Engine/EngineDebugMaterials/VertexColorViewMode_ColorOnly.VertexColorViewMode_ColorOnly" :`NewEnumerator1` "/Game/StaticMeshes/Blockout/TeamBlueEmissive.TeamBlueEmissive" :`NewEnumerator2` "/Engine/EngineDebugMaterials/VertexColorViewMode_GreenOnly.VertexColorViewMode_GreenOnly" :!type "MaterialInterface Object Reference")))